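; Laser eye hazard that kills the player after keeping line of sight for a charge time.
; Each Tick, while the player controller has line of sight, it aims a visible beam at the pawn and starts a one-shot timer through a DoOnce.
; Losing sight hides the beam, clears the timer and resets the DoOnce.
; On expiry, a timeline scales the beam, then calls Death on Runner_PlayerController without rechecking sight.
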(event Custom|FireLaser
  ;[1 1 1] Check for LOS to player, if true start fire timer. Timer stops if LOS is broken
  (bind _newtrack_0 (Timeline|LaserScale PlayFromStart)
    (:Update
      (Transformation|SetRelativeScale3D (Variables|Default|GetLaserEmit) (Math|Vector|MakeVector _newtrack_0 _newtrack_0 _newtrack_0)))
    (:Finished
      (bind _asrunner_player_controller (Utilities|Casting|CastToRunner_PlayerController (Game|GetPlayerController 0)))
      (Default|Death _asrunner_player_controller))))

(event EventBeginPlay)

(event Collision|EventActorBeginOverlap
  (params (OtherActor :type Actor%20Object%20Reference)))

(event EventTick
  (params (DeltaSeconds :type Float%20%28single-precision%29))
  ;[1 1 1] Check for LOS to player, if true start fire timer. Timer stops if LOS is broken
  (if (Controller|LineOfSightTo (Game|GetPlayerController 0) self "0, 0, 0" false)
    (Rendering|SetVisibility (Variables|Default|GetLaserEmit) true false)
    (Class|ParticleSystemComponent|SetBeamSourcePoint (Variables|Default|GetLaserEmit) 0 (Transformation|GetWorldLocation (Variables|Default|GetRenderComponent)))
    (Class|ParticleSystemComponent|SetBeamTargetPoint (Variables|Default|GetLaserEmit) 0 (Transformation|GetActorLocation (Game|Player|GetPlayerPawn 0)))
    (Utilities|FlowControl|DoOnce false :!label _label
      (:Completed
        (bind _returnvalue (Utilities|Time|SetTimerbyEvent (delegate Custom|FireLaser) (Variables|Default|GetChargeTime)))
        (Variables|Default|SetCurrentTimer _returnvalue)))
    (else
      (Rendering|SetVisibility (Variables|Default|GetLaserEmit) false false)
      (Utilities|Time|ClearandInvalidateTimerbyHandle (Variables|Default|GetCurrentTimer))
      (goto _label Reset))))

(fn ConstructionScript)