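; Player controller for a runner game that tracks opener collection, level restarts and level progression.
; BeginPlay caches all openers and doors; Tick activates every door each frame while the externally updated collected count equals the total.
; Otherwise, holding R for over half a second reloads the level.
; LevelComplete shows a widget, stops the cube pawn and pauses after short delays, while NextLevel opens the following entry in Levels.
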(event Custom|LevelComplete
  (bind _returnvalue (UserInterface|CreateWidget "/Game/UI/LevelComplete_Widget.LevelComplete_Widget_C"))
  (UserInterface|Viewport|AddtoViewport _returnvalue 0)
  (Utilities|FlowControl|Delay 0.05)
  (bind _ascube_bp (Utilities|Casting|CastToCube_BP (Game|Player|GetPlayerPawn 0)))
  (Default|StopVelocity _ascube_bp)
  (Utilities|FlowControl|Delay 0.7)
  (Game|SetGamePaused true))

(event Custom|NextLevel
  (bind _returnvalue (Game|GetCurrentLevelName true))
  (if (<= (+ (Utilities|Array|FindItem (Variables|Default|GetLevels) (Utilities|String|StringToName _returnvalue)) 1) (Utilities|Array|LastIndex (Variables|Default|GetLevels)))
    (Game|OpenLevel(byName) (Utilities|Array|Get(acopy) (Variables|Default|GetLevels) (+ (Utilities|Array|FindItem (Variables|Default|GetLevels) (Utilities|String|StringToName _returnvalue)) 1)))))

(event EventBeginPlay
  (bind _outactors (Actor|GetAllActorsOfClass "/Game/Blueprints/Opener_BP.Opener_BP_C"))
  (bind _output_get (Variables|Default|SetOpeners _outactors))
  (Variables|Default|SetNumOpeners (Utilities|Array|Length _output_get))
  (bind _outactors_2 (Actor|GetAllActorsOfClass "/Game/Blueprints/Door_BP.Door_BP_C"))
  (Variables|Default|SetDoors _outactors_2))

(event EventTick
  (params (DeltaSeconds :type Float%20%28single-precision%29))
  (if (== (Variables|Default|GetCollectedOpeners) (Variables|Default|GetNumOpeners))
    (for _array_element (Variables|Default|GetDoors)
      (Default|ActivateDoor _array_element))
    (elif (> (Class|PlayerController|GetInputKeyTimeDown "R") 0.5)
      (bind _returnvalue (Game|GetCurrentLevelName true))
      (Game|OpenLevel(byName) (Utilities|String|StringToName _returnvalue)))))

(fn ConstructionScript)