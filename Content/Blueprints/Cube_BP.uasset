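; Cube_BP is a side-scrolling Paper2D player character that runs along world X, jumps and turns to face its input direction.
; Input drives movement and flips player controller 0's yaw between 0 and 180.
; Each tick, velocity and falling state feed AnimationStateMachine, a simple function that selects the idle, run or non-looping jump flipbook.
; The sprite component is set to replicate on BeginPlay.
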(event Custom|UpdateAnimation
  (bind _sprite (Variables|Default|GetSprite))
  (bind _output_get (Variables|Default|SetIsMoving (> (Math|Vector|VectorLength (Transformation|GetVelocity)) 0.0)))
  (bind _output_get_2 (Variables|Default|SetIsFalling (AI|Components|NavMovement|IsFalling (Variables|Character|GetCharacterMovement))))
  (bind _outputflipbook (CallFunction|AnimationStateMachine _output_get_2 _output_get))
  (Sprite|SetFlipbook _sprite _outputflipbook)
  (Audio|Components|Audio|Play _sprite))

(event EventBeginPlay
  (Class|ActorComponent|SetIsReplicated (Variables|Default|GetSprite) true))

(event Collision|EventActorBeginOverlap
  (params (OtherActor :type Actor%20Object%20Reference)))

(event EventTick
  (params (DeltaSeconds :type Float%20%28single-precision%29))
  (CallFunction|UpdateAnimation))

(event Input|ActionEvents|InputActionJump
  (params (Key :type Key%20Structure))
  (:Pressed
    (Character|Jump)))

(event Input|AxisEvents|InputAxisMoveRight
  (params (AxisValue :type Float%20%28single-precision%29))
  (Pawn|Input|AddMovementInput "1.000000, 0, 0" AxisValue false)
  (Math|Float|CompareFloat AxisValue 0.0
    (:>
      (Pawn|SetControlRotation (Game|GetPlayerController 0) (Math|Rotator|MakeRotator 0.0 0.0 0.0)))
    (:<
      (Pawn|SetControlRotation (Game|GetPlayerController 0) (Math|Rotator|MakeRotator 0.0 0.0 1.8e+02)))))

(fn ConstructionScript)

(fn AnimationStateMachine
  (params (IsFalling :type Boolean) (IsMoving :type Boolean))
  (if (Variables|Default|GetIsFalling)
    (Components|Timeline|SetLooping (Variables|Default|GetSprite) false)
    (LocalVariables|SetAnimationState "NewEnumerator2")
    (else
      (Components|Timeline|SetLooping (Variables|Default|GetSprite) true)
      (if (Variables|Default|GetIsMoving)
        (LocalVariables|SetAnimationState "NewEnumerator1")
        (else
          (LocalVariables|SetAnimationState "NewEnumerator0")))))
  (return (Utilities|Select :Index (LocalVariables|GetAnimationState) :NewEnumerator0 (Variables|Animations|GetIdle_Flipbook) :NewEnumerator1 (Variables|Animations|GetRun_Flipbook) :NewEnumerator2 (Variables|Animations|GetJump_Flipbook))))